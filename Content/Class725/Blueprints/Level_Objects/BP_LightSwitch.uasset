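; BP_LightSwitch is a level object that lets an interaction turn a referenced scene light on and off.
; On BeginPlay it binds its handler to the interaction event dispatcher of its CBPInteractable component.
; Each interaction alternates through a FlipFlop, starting with on, setting the light's intensity and snapping the Button between two relative positions to match.
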(event `self.ReceiveBeginPlay`
  (add `/Game/Class725/Components/CBP_Interactable.ED_Interaction` (`self.CBP_Interactable`) (delegate `Interaction Event`)))

(event `Interaction Event`
  (`/Engine/EditorBlueprintResources/StandardMacros.FlipFlop`
    (:`A`
      (`LightComponent.SetIntensity` (`Light.LightComponent` (`self.Light in Scene`)) 15.0)
      (`SceneComponent.K2_SetRelativeLocation` (`self.Button`) (0.0 0.0 0.0) false false))
    (:`B`
      (`LightComponent.SetIntensity` (`Light.LightComponent` (`self.Light in Scene`)) 0.0)
      (`SceneComponent.K2_SetRelativeLocation` (`self.Button`) (0.0 0.0 10.0) false false))))

(fn `UserConstructionScript`)